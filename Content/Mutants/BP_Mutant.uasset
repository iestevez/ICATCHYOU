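; BP_Mutant is an AI-driven mutant that turns into a killer after a random delay and destroys itself after a random lifetime.
; On BeginPlay it clears the killer blackboard flag, randomizes both timers within min/max ranges and sets its starting material.
; When the kill timer ends, it swaps material and sets the flag.
; PawnSensing writes any seen BP_Pawn to the blackboard as the player pawn.
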(event OnSeePawn(PawnSensing)
  (params (Pawn :type Pawn%20Object%20Reference))
  (bind _blackboard (Variables|Blackboard|GetBlackboard))
  (bind _asbp_pawn (Utilities|Casting|CastToBP_Pawn Pawn))
  (Utilities|IsValid _blackboard
    (:Is%20Valid
      (AI|Components|Blackboard|SetValueasObject _blackboard (Variables|Blackboard|GetPlayerPawnKey) _asbp_pawn))))

(event EventBeginPlay
  (bind _output_get (Variables|Blackboard|SetBlackboard (AI|GetBlackboard 0)))
  (Utilities|IsValid _output_get
    (:Is%20Valid
      (AI|Components|Blackboard|SetValueasBool _output_get (Variables|Blackboard|GetKillerStateKey) false)
      (Utilities|RandomizeParameters
        (:Out
          (Utilities|FlowControl|Sequence
            (:then_0
              (Rendering|Material|SetMaterial (Variables|Default|GetStaticMesh) 0 "/Engine/MapTemplates/Materials/BasicAsset03.BasicAsset03"))
            (:then_1
              (Utilities|FlowControl|Delay (Variables|MutantBehaviour|GetTimeToKill))
              (Rendering|Material|SetMaterial (Variables|Default|GetStaticMesh) 0 "/Engine/MapTemplates/Materials/BasicAsset01.BasicAsset01")
              (Utilities|IsValid (Variables|Blackboard|GetBlackboard)
                (:Is%20Valid
                  (AI|Components|Blackboard|SetValueasBool (Variables|Blackboard|GetBlackboard) (Variables|Blackboard|GetKillerStateKey) true))))
            (:then_2
              (Utilities|FlowControl|Delay (Variables|MutantBehaviour|GetLifeTime))
              (Actor|DestroyActor))))))))

(event Collision|EventActorBeginOverlap
  (params (OtherActor :type Actor%20Object%20Reference)))

(event EventTick
  (params (DeltaSeconds :type Float%20%28single-precision%29)))

(fn ConstructionScript)