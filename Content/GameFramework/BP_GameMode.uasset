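; Game mode that manages lives and the end-of-game flow for the player pawn.
; It copies its Lifes value to BP_Pawn at BeginPlay and sets BP_Pawn as the default pawn class when the main level starts.
; LifeLost calls EndGame once the pawn's lives equal zero.
; EndGame destroys the Spawner, freezes the pawn and passes its points as an integer to BP_Hud's GameFinished.
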(event Custom|LifeLost
  (bind _asbp_pawn (Utilities|Casting|CastToBP_Pawn (Game|Player|GetPlayerPawn 0)))
  (if (== (Variables|/Game/GameFramework/BP_Pawn.BP_Pawn_C|GetLifes _asbp_pawn) 0)
    (Utilities|EndGame)))

(event Custom|OnMainLevelStarted
  (Variables|Default|SetDefaultPawnClass "/Game/GameFramework/BP_Pawn.BP_Pawn_C"))

(event EventBeginPlay
  (bind _asbp_pawn (Utilities|Casting|CastToBP_Pawn (Game|Player|GetPlayerPawn 0)))
  (Variables|/Game/GameFramework/BP_Pawn.BP_Pawn_C|SetLifes _asbp_pawn (Variables|Default|GetLifes)))

(event EventTick
  (params (DeltaSeconds :type Float%20%28single-precision%29)))

(fn ConstructionScript)